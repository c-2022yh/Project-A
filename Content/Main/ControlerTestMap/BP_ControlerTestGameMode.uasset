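; Test game mode for a tile-board battle with preparation and combat phases.
; On BoardReady it spawns a hard-coded enemy and two player units, registers them on tiles or in the waiting area, then starts preparation.
; Phase events create the battle HUD, start combat on request or timeout, and dispatch results and restarts.
; SpawnRosterUnits offers roster-driven setup within the same begin/complete/cancel encounter bracket, but is not called here.
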(event EventBeginPlay)

(event EventBoardReady
  (bind _returnvalue (Class|AutoBattleGameMode|BeginEncounterSetup))
  (if _returnvalue
    (bind _returnvalue_2 (Game|SpawnActorfromClass "/Script/Project_A.BattleUnitBase" (Math|Transform|MakeTransform (Transformation|GetActorLocation (Variables|Default|GetBoardManager))) "AlwaysSpawn" "MultiplyWithRoot" 0 0))
    (Variables|/Script/Project_A.BattleUnitBase|SetTeamType _returnvalue_2 "Enemy")
    (bind _returnvalue_3 (Class|AutoBattleGameMode|RegisterBattleUnit _returnvalue_2))
    (if _returnvalue_3
      (bind _returnvalue_4 (Class|BattleUnitBase|PlaceonTile _returnvalue_2 (Class|BoardManager|GetTile (Variables|Default|GetBoardManager) 4 1)))
      (if _returnvalue_4
        (bind _returnvalue_5 (Game|SpawnActorfromClass "/Script/Project_A.BattleUnitBase" (Math|Transform|MakeTransform (Transformation|GetActorLocation (Variables|Default|GetBoardManager))) "AlwaysSpawn" "MultiplyWithRoot" 0 0))
        (Variables|/Script/Project_A.BattleUnitBase|SetTeamType _returnvalue_5 "Player")
        (bind _returnvalue_6 (Class|AutoBattleGameMode|RegisterBattleUnit _returnvalue_5))
        (if _returnvalue_6
          (bind _returnvalue_7 (Class|BattleUnitBase|PlaceonTile _returnvalue_5 (Class|BoardManager|GetTile (Variables|Default|GetBoardManager) 0 1)))
          (if _returnvalue_7
            (bind _returnvalue_8 (Game|SpawnActorfromClass "/Script/Project_A.BattleUnitBase" (Math|Transform|MakeTransform (Transformation|GetActorLocation (Variables|Default|GetBoardManager))) "AlwaysSpawn" "MultiplyWithRoot" 0 0))
            (Variables|/Script/Project_A.BattleUnitBase|SetTeamType _returnvalue_8 "Player")
            (bind _returnvalue_9 (Class|AutoBattleGameMode|RegisterBattleUnit _returnvalue_8))
            (if _returnvalue_9
              (bind _returnvalue_10 (Class|AutoBattleGameMode|MoveUnittoWaitingArea _returnvalue_8 0 1))
              (if _returnvalue_10
                (bind _returnvalue_11 (Class|AutoBattleGameMode|CompleteEncounterSetup))
                (if _returnvalue_11
                  (Class|AutoBattleGameMode|StartPreparationPhase))))))))))

(event EventCombatStartRequested
  (Class|AutoBattleGameMode|StartCombatPhase))

(event EventPreparationExpired
  (Class|AutoBattleGameMode|RequestCombatStart))

(event EventBattleResultDetected
  (params (Result :type EGamePhase%20Enum :default "Preparation"))
  (switch Utilities|FlowControl|Switch|SwitchonEGamePhase "Preparation"
    (:RoundClear
      (Class|AutoBattleGameMode|HandleRoundClear))
    (:GameOver
      (Class|AutoBattleGameMode|HandleGameOver))
    (:Victory
      (Class|AutoBattleGameMode|HandleVictory))))

(event EventRestartRequested
  (Class|AutoBattleGameMode|RestartBattle))

(event EventGamePhaseChanged
  (params (Phase :type EGamePhase%20Enum :default "Preparation"))
  (switch Utilities|FlowControl|Switch|SwitchonEGamePhase Phase
    (:Preparation
      (Utilities|IsValid (Variables|Default|GetBattleHUD)
        (:Is%20Valid
          _)
        (:Is%20Not%20Valid
          _))
      (bind _returnvalue (UserInterface|CreateWidget "/Game/BluePrints/Widget/WBP_BattleHUD.WBP_BattleHUD_C" (Game|GetPlayerController 0)))
      (Variables|Default|SetBattleHUD _returnvalue)
      (UserInterface|Viewport|AddtoViewport _returnvalue 0))))

(fn ConstructionScript)

(fn SpawnRosterUnits
  (Variables|Default|SetWaitingCount 0)
  (Variables|Default|SetWaitingIndex 0)
  (Variables|Default|SetSpawnSucceeded true)
  (bind _returnvalue (Class|AutoBattleGameMode|BeginEncounterSetup))
  (if _returnvalue
    (for _array_element (Variables|Default|GetUnitRoster)
      (if (and (Utilities|Enum|Equal(Enum) (.Team (Utilities|Struct|BreakUnitSpawnInfo _array_element)) "Player") (not (.bStartOnBoard (Utilities|Struct|BreakUnitSpawnInfo _array_element))))
        (Variables|Default|SetWaitingCount (+ (Variables|Default|GetWaitingCount) 1))))
    (bind _array_element_2 (Utilities|Array|ForEachLoopwithBreak (Variables|Default|GetUnitRoster) :!label _label)
      (:LoopBody
        (bind _returnvalue_2 (Game|SpawnActorfromClass (.UnitClass (Utilities|Struct|BreakUnitSpawnInfo _array_element_2)) (Math|Transform|MakeTransform (Transformation|GetActorLocation (Variables|Default|GetBoardManager))) "AlwaysSpawn" "MultiplyWithRoot" 0 0))
        (Variables|/Script/Project_A.BattleUnitBase|SetTeamType _returnvalue_2 (.Team (Utilities|Struct|BreakUnitSpawnInfo _array_element_2)))
        (bind _returnvalue_3 (Class|AutoBattleGameMode|RegisterBattleUnit _returnvalue_2))
        (if _returnvalue_3
          (if (.bStartOnBoard (Utilities|Struct|BreakUnitSpawnInfo _array_element_2))
            (bind _returnvalue_4 (Class|BattleUnitBase|PlaceonTile _returnvalue_2 (Class|BoardManager|GetTile (Variables|Default|GetBoardManager) (.Row (Utilities|Struct|BreakUnitSpawnInfo _array_element_2)) (.Column (Utilities|Struct|BreakUnitSpawnInfo _array_element_2)))))
            (if (not _returnvalue_4)
              (bind _output_get (Variables|Default|SetSpawnSucceeded true))
              (Class|AutoBattleGameMode|CancelEncounterSetup)
              (goto _label Break))
            (else
              (bind _returnvalue_5 (Class|AutoBattleGameMode|MoveUnittoWaitingArea _returnvalue_2 (Variables|Default|GetWaitingIndex) (Variables|Default|GetWaitingCount)))
              (if _returnvalue_5
                (Variables|Default|SetWaitingCount (+ (Variables|Default|GetWaitingCount) 1)))))))
      (:Completed
        (if _output_get
          (bind _returnvalue_6 (Class|AutoBattleGameMode|CompleteEncounterSetup))
          (if _returnvalue_6
            (return true)
            (else
              (Class|AutoBattleGameMode|CancelEncounterSetup)
              (return false)))
          (else
            (return false)))))
    (else
      (return false))))