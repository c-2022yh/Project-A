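; BP_UnitBase is a base unit Blueprint that handles the visuals for projectiles and shields.
; Projectile update events spawn a BP_UnitProjectileVisual on first sight of an ID, apply its mesh visual, then move that actor to the reported transform.
; The actors are tracked in an ID-keyed map and destroyed on removal.
; A shield-changed binding, set at BeginPlay, shows the shield mesh only while CurrentShield is above zero.
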(event Custom|UpdateShieldVisual
  (params (Unit :type Battle%20Unit%20Base%20Object%20Reference))
  (Rendering|SetVisibility (Variables|Default|GetShieldVisual) (> (Variables|/Script/Project_A.BattleUnitBase|GetCurrentShield Unit) 0.0) false))

(event EventBeginPlay
  (EventDispatchers|BindEventtoOnShieldChanged (delegate Custom|UpdateShieldVisual)))

(event Collision|EventActorBeginOverlap
  (params (OtherActor :type Actor%20Object%20Reference)))

(event EventTick
  (params (DeltaSeconds :type Float%20%28single-precision%29)))

(event EventProjectileUpdated
  (params (Projectile :type Unit%20Projectile%20View%20Structure%20%28by%20ref%29))
  (bind _projectilevisuals (Variables|Default|GetProjectileVisuals))
  (bind (_value _returnvalue) (Utilities|Map|Find _projectilevisuals (.projectileid Projectile)))
  (if _returnvalue
    (Transformation|SetActorLocationAndRotation _value (.position Projectile) (.rotation Projectile))
    (else
      (bind _returnvalue_2 (Game|SpawnActorfromClass "/Game/BluePrints/Units/Projectiles/BP_UnitProjectileVisual.BP_UnitProjectileVisual_C" (Math|Transform|MakeTransform (.position Projectile) (.rotation Projectile) "1.000000,1.000000,1.000000") "AlwaysSpawn" "MultiplyWithRoot" 0 0))
      (Class|UnitProjectileVisualLibrary|ApplyProjectileVisual (Variables|/Game/BluePrints/Units/Projectiles/BP_UnitProjectileVisual.BP_UnitProjectileVisual_C|GetProjectileMesh _returnvalue_2) (.visual Projectile))
      (Utilities|Map|Add _projectilevisuals (.projectileid Projectile) _returnvalue_2))))

(event EventProjectileRemoved
  (params (ProjectileId :type Integer) (bHit :type Boolean))
  (bind _projectilevisuals (Variables|Default|GetProjectileVisuals))
  (bind _value (Utilities|Map|Find _projectilevisuals ProjectileId))
  (Utilities|IsValid _value
    (:Is%20Valid
      (Actor|DestroyActor _value))
    (:Is%20Not%20Valid
      _))
  (Utilities|Map|Remove _projectilevisuals ProjectileId))

(fn ConstructionScript)