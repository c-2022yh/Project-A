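; Base unit Blueprint that handles the visual side of a unit's projectiles and shield.
; Projectile update events spawn or move a BP_UnitProjectileVisual actor tracked in a map by projectile ID, drawing non-basic attacks at double scale.
; Projectile removal events destroy that actor and clear its map entry.
; On BeginPlay it binds to OnShieldChanged, showing the shield visual only while current shield is above zero.
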(event Custom|UpdateShieldVisual
  (params (Unit :type Battle%20Unit%20Base%20Object%20Reference))
  (Rendering|SetVisibility (Variables|Default|GetShieldVisual) (> (Variables|/Script/Project_A.BattleUnitBase|GetCurrentShield Unit) 0.0) false))

(event EventBeginPlay
  (EventDispatchers|BindEventtoOnShieldChanged (delegate Custom|UpdateShieldVisual)))

(event Collision|EventActorBeginOverlap
  (params (OtherActor :type Actor%20Object%20Reference)))

(event EventTick
  (params (DeltaSeconds :type Float%20%28single-precision%29)))

(event EventProjectileUpdated
  (params (Projectile :type Unit%20Projectile%20View%20Structure%20%28by%20ref%29))
  (bind _returnvalue (Math|Float|SelectFloat 1.0 2.0 (.bbasicattack Projectile)))
  (bind _projectilevisuals (Variables|Default|GetProjectileVisuals))
  (bind (_value _returnvalue_2) (Utilities|Map|Find _projectilevisuals (.projectileid Projectile)))
  (if _returnvalue_2
    (Transformation|SetActorLocation _value (.position Projectile) false false)
    (else
      (bind _returnvalue_3 (Game|SpawnActorfromClass "/Game/BluePrints/Units/Projectiles/BP_UnitProjectileVisual.BP_UnitProjectileVisual_C" (Math|Transform|MakeTransform (.position Projectile) "0, 0, 0" (Math|Vector|MakeVector _returnvalue _returnvalue _returnvalue)) "AlwaysSpawn" "MultiplyWithRoot" 0 0))
      (Utilities|Map|Add _projectilevisuals (.projectileid Projectile) _returnvalue_3))))

(event EventProjectileRemoved
  (params (ProjectileId :type Integer) (bHit :type Boolean))
  (bind _projectilevisuals (Variables|Default|GetProjectileVisuals))
  (bind _value (Utilities|Map|Find _projectilevisuals ProjectileId))
  (Utilities|IsValid _value
    (:Is%20Valid
      (Actor|DestroyActor _value))
    (:Is%20Not%20Valid
      _))
  (Utilities|Map|Remove _projectilevisuals ProjectileId))

(fn ConstructionScript)