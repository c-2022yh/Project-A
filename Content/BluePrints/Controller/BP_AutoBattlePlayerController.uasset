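; Player controller for the auto-battle mode that handles mouse-driven dragging of battle units on the board.
; On BeginPlay it configures drag tuning, shows the cursor in Game and UI input mode, and blends the view to the actor tagged BattleCamera.
; Pressing left mouse traces the board and begins dragging any BattleUnitBase hit; releasing ends the drag and clears the selection.
; Input uses debug key events, and drag functions are called, not implemented, here.
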(event EventBeginPlay
  (Variables|Default|SetUnitDragHeightOffset 4e+02)
  (Variables|Default|SetUnitDragThreshold 12.0)
  (Input|SetInputModeGameandUI self 0 "DoNotLock" false false)
  (Variables|Default|SetbShowMouseCursor true)
  (bind _outactors (Actor|GetAllActorsOfClasswithTag 0 "BattleCamera"))
  (Utilities|IsValid (Utilities|Array|Get(acopy) _outactors)
    (:Is%20Valid
      (Game|Player|SetViewTargetwithBlend (Utilities|Array|Get(acopy) _outactors) 0.0 "VTBlend_Linear" 0.0 false))))

(event Input|MouseEvents|DebugKeyLeftMouseButton
  (params (Key :type Key%20Structure :default "None") (ActionValue :type Input%20Action%20Value%20Structure))
  (:Pressed
    (bind (_hit _returnvalue) (Class|AutoBattlePlayerController|GetBoardClickHit))
    (if _returnvalue
      (bind _asbattle_unit_base (Utilities|Casting|CastToBattleUnitBase (.HitActor (Collision|BreakHitResult _hit))))
      (Class|AutoBattlePlayerController|BeginUnitDrag _asbattle_unit_base)))
  (:Released
    (Class|AutoBattlePlayerController|EndUnitDrag)
    (Class|AutoBattlePlayerController|ClearSelection)))

(fn ConstructionScript)